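; SpawnBP is an actor that spawns and scatters a head pickup when a CharacterBP overlaps it.
; The overlap calls Spawn on HeadPickupSpawn, randomly rotates the new mesh and prints that rotation.
; A radial impulse from a randomly offset point near the spawn location then launches the mesh.
; A looping timer event shares this spawn path, but the timer setup is disconnected, so only overlaps trigger spawning.
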(event `self.ReceiveActorBeginOverlap`
  (params (OtherActor :type "Actor Object Reference"))
  (bind _headpickupspawn (`self.HeadPickupSpawn`))
  (cast `/Game/Character/Blueprint/CharacterBP` OtherActor)
  (bind _returnvalue (`HeadPickupSpawn.Spawn` _headpickupspawn :!label _label))
  (bind _mesh (`Pickup.Mesh` _returnvalue))
  (`SceneComponent.K2_SetWorldRotation` _mesh (`KismetMathLibrary.RandomRotator` false) false)
  (`KismetSystemLibrary.PrintString` (`KismetStringLibrary.Conv_RotatorToString` (`SceneComponent.K2_GetComponentRotation` _mesh)))
  (`PrimitiveComponent.AddRadialImpulse` _mesh (`KismetMathLibrary.MakeVector` (+ (.x (`SceneComponent.K2_GetComponentLocation` _headpickupspawn)) (`KismetMathLibrary.RandomFloatInRange` -50.0 50.0)) (+ (.y (`SceneComponent.K2_GetComponentLocation` _headpickupspawn)) (`KismetMathLibrary.RandomFloatInRange` -50.0 50.0)) (+ (.z (`SceneComponent.K2_GetComponentLocation` _headpickupspawn)) (`KismetMathLibrary.RandomFloatInRange` -50.0 50.0))) 200.0 50000.0 "RIF_Linear" false))

(event `self.ReceiveBeginPlay`)

(event `SpawnTimer`
  (goto _label))

(fn `UserConstructionScript`)